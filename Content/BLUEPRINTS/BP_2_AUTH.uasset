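; Authentication controller that runs the player sign-in flow through FastGameSubsystem and opens the next level once authenticated.
; On BeginPlay it checks existing auth, otherwise shows the WDGT_AUTH widget in UI-only input mode.
; Entering an ID branches to password, account completion, OTP verification or registration pages, with events handling signup, code checks and password confirmation.
; Failures only print debug messages, and exit clears the cached identity.
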(event Custom|NextLevel
  ;[5.8e-05 0.1343 0.15 0.5] NEXT_LEVEL
  (Development|PrintString "AUTHENTICATED" true true "(R=0.000000,G=0.660000,B=1.000000,A=1.000000)" (.debug_duration (Variables|Default|GetBUILD_SETTINGS)))
  (Game|OpenLevel(byObjectReference) (Variables|Default|GetNEXT_SCENE)))

(event Custom|EXIT
  (bind _returnvalue (Subsystems|GetFastGameSubsystem))
  ;[0.1007 0 0.15 0.5] EXIT
  (Class|FastGameSubsystem|ClearEnteredIdentity _returnvalue)
  (Class|FastGameSubsystem|ClearLocalCache _returnvalue)
  (Default|ENTERIDPAGE (Variables|Default|GetAUTH))
  (Development|PrintString "EXIT" true true "(R=0.000000,G=0.660000,B=1.000000,A=1.000000)" (.debug_duration (Variables|Default|GetBUILD_SETTINGS))))

(event Custom|LOGIN
  ;[0.15 0 0.09718 0.5] LOGIN
  (Development|PrintString "ENTER" true true "(R=0.000000,G=0.660000,B=1.000000,A=1.000000)" (.debug_duration (Variables|Default|GetBUILD_SETTINGS)))
  (bind _returnvalue (UserInterface|CreateWidget "/Game/ART/UI/WIDGETS/WDGT_AUTH.WDGT_AUTH_C" (Game|GetPlayerController 0)))
  (UserInterface|Viewport|AddtoPlayerScreen _returnvalue)
  (Input|SetInputModeUIOnly (Game|GetPlayerController 0) 0 "DoNotLock" false)
  (CallFunction|SETREFS)
  (Default|ENTERIDPAGE (Variables|Default|GetAUTH)))

(event Custom|SET_REFS
  ;[0.0161 0 0.15 0.5] SET_REFS
)

(event Custom|SEND_OTP_CODE
  ;[0 0.15 0.03331 0.5] SEND/RESEND OTP
  (bind (_bsuccess _statuscode _message) (Class|FastGameSubsystem|SendAuthCode (Subsystems|GetFastGameSubsystem)))
  (if _bsuccess
    (Default|OTPPAGE (Variables|Default|GetAUTH))
    (else
      (Development|PrintString _message true true "(R=0.000000,G=0.660000,B=1.000000,A=1.000000)" (.debug_duration (Variables|Default|GetBUILD_SETTINGS))))))

(event Custom|ENTER
  (params (ID :type String))
  (bind _build_settings (Variables|Default|GetBUILD_SETTINGS))
  (bind _auth (Variables|Default|GetAUTH))
  ;[0.15 0.13 0 0.5] ENTER
  (bind _message (Class|FastGameSubsystem|Enter (Subsystems|GetFastGameSubsystem) ID (.id_channel _build_settings))
    (:Login
      (Default|ENTERPASSWORDPAGE _auth))
    (:CompleteAccount
      (Default|NEWPASSPAGE _auth))
    (:VerifyId
      (CallFunction|SENDOTPCODE))
    (:Register
      (Default|REGISTERPAGE _auth))
    (:Failed
      (Development|PrintString _message true true "(R=0.000000,G=0.660000,B=1.000000,A=1.000000)" (.debug_duration _build_settings)))))

(event Custom|REGISTER
  (params (FULL_NAME :type String) (PASSWORD :type String) (CONFIRM_PASS :type String))
  ;[0.0183 0.15 0 0.5] REGISTER
  (bind (_bsuccess _statuscode _userid _outemail _outphone _message) (Class|FastGameSubsystem|Signup (Subsystems|GetFastGameSubsystem) "" "" PASSWORD CONFIRM_PASS FULL_NAME))
  (if _bsuccess
    (CallFunction|NextLevel)
    (else
      (Development|PrintString _message true true "(R=0.000000,G=0.660000,B=1.000000,A=1.000000)" (.debug_duration (Variables|Default|GetBUILD_SETTINGS))))))

(event Custom|VERIFY
  (params (CODE :type String))
  ;[0 0.1369 0.15 0.5] VERIFY
  (bind (_bsuccess _statuscode _message) (Class|FastGameSubsystem|VerifyAuthCode (Subsystems|GetFastGameSubsystem) "" CODE))
  (if _bsuccess
    (Default|NEWPASSPAGE (Variables|Default|GetAUTH))
    (else
      (Development|PrintString _message true true "(R=0.000000,G=0.660000,B=1.000000,A=1.000000)" (.debug_duration (Variables|Default|GetBUILD_SETTINGS))))))

(event Custom|NEW_PASS
  (params (PASSWORD :type String) (CONFIRM_PASS :type String))
  ;[0 0.06215 0.15 0.5] NEW_PASS
  (bind (_bsuccess _statuscode _message) (Class|FastGameSubsystem|ConfirmPasswordRecovery (Subsystems|GetFastGameSubsystem) "" PASSWORD CONFIRM_PASS))
  (if _bsuccess
    (CallFunction|NextLevel)
    (else
      (Development|PrintString _message true true "(R=0.000000,G=0.660000,B=1.000000,A=1.000000)" (.debug_duration (Variables|Default|GetBUILD_SETTINGS))))))

(event EventBeginPlay
  (bind _build_settings (Variables|Default|GetBUILD_SETTINGS))
  ;[0.15 0.003394 0 0.5] INIT_CHECK_AUTH => NEXT LEVEL OR LOGIN
  (Development|PrintString "INITIALIZED AUTH" true true "(R=0.000000,G=0.660000,B=1.000000,A=1.000000)" (.debug_duration _build_settings))
  (bind (_bsuccess _statuscode _message _bauthenticated) (Class|FastGameSubsystem|CheckAuthentication (Subsystems|GetFastGameSubsystem)))
  (if _bsuccess
    (if _bauthenticated
      (CallFunction|NextLevel)
      (else
        (Development|PrintString _message true true "(R=0.000000,G=0.660000,B=1.000000,A=1.000000)" (.debug_duration _build_settings))
        (CallFunction|LOGIN)))
    (else
      (Development|PrintString _message true true "(R=0.000000,G=0.660000,B=1.000000,A=1.000000)" (.debug_duration _build_settings)))))

(fn ConstructionScript)