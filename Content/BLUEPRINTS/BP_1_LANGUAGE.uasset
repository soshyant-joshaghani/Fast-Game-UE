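; BP_1_LANGUAGE is the language selection scene Blueprint that shows the language widget and moves on to the next level.
; On BeginPlay it creates WDGT_LANGUAGE, adds it to the player screen and switches input to UI only.
; The NextLevel event receives LANG, only prints it without storing it, then opens NEXTSCENE by object reference.
; Debug print durations come from BUILDSETTINGS.
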(event Custom|NextLevel
  (params (LANG :type String))
  ;[0.15 0.15 0.15 0.5] NEXT_LEVEL
  (Development|PrintString LANG true true "(R=0.000000,G=0.660000,B=1.000000,A=1.000000)" (.debug_duration (Variables|Default|GetBUILD_SETTINGS)))
  (Game|OpenLevel(byObjectReference) (Variables|Default|GetNEXT_SCENE)))

(event EventBeginPlay
  ;[0.15 0.1299 0.03088 0.5] INITIALIZE
  (Development|PrintString "BP_LANGUAGE_INITIALIZED" true true "(R=0.000000,G=0.660000,B=1.000000,A=1.000000)" (.debug_duration (Variables|Default|GetBUILD_SETTINGS)))
  (bind _returnvalue (UserInterface|CreateWidget "/Game/ART/UI/WIDGETS/WDGT_LANGUAGE.WDGT_LANGUAGE_C" (Game|GetPlayerController 0)))
  (UserInterface|Viewport|AddtoPlayerScreen _returnvalue)
  (Input|SetInputModeUIOnly (Game|GetPlayerController 0) 0 "DoNotLock" false))

(event Collision|EventActorBeginOverlap
  (params (OtherActor :type Actor%20Object%20Reference)))

(event EventTick
  (params (DeltaSeconds :type Float%20%28single-precision%29)))

(fn ConstructionScript)