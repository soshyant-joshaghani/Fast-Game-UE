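; Splash-screen Blueprint that boots the game, shows a splash widget and then loads the next level.
; On BeginPlay it initializes the game through FastGameSubsystem with game code and store platform, then the API client, printing failure messages.
; It then shows WDGT_SPLASH with UI-only input, waits briefly and opens NEXTSCENE.
; Initialization failures do not stop the transition to the next level.
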(event Custom|NextLevel
  ;[0.02435 0.03889 0.15 0.5] NEXT_LEVEL
  (Game|OpenLevel(byObjectReference) (Variables|Default|GetNEXT_SCENE)))

(event EventBeginPlay
  (bind _returnvalue (Game|GetPlayerController 0))
  (bind _bs (Variables|Default|GetBS))
  (Development|PrintString "BP_SPLASH_INITIALIZED" true true "(R=0.000000,G=0.660000,B=1.000000,A=1.000000)" (.debug_duration (Variables|Default|GetBS)))
  (Utilities|FlowControl|Sequence
    (:then_0
      ;[0.15 0.1257 0.02089 0.5] INITIALIZE
      (Development|PrintString "INITIALIZE GAME" true true "(R=0.000000,G=0.660000,B=1.000000,A=1.000000)" (.debug_duration _bs))
      (bind (_bsuccess _message) (Class|FastGameSubsystem|InitializeGame (Subsystems|GetFastGameSubsystem) (.game_code _bs) (.platform _bs)))
      (if _bsuccess
        (bind (_bsuccess_2 _message_2) (Class|FastGameSubsystem|InitializeClient (Subsystems|GetFastGameSubsystem) (.api_base_url _bs)))
        (if (not _bsuccess_2)
          (Development|PrintString _message_2 true true "(R=0.000000,G=0.660000,B=1.000000,A=1.000000)" (.debug_duration _bs)))
        (else
          (Development|PrintString _message true true "(R=0.000000,G=0.660000,B=1.000000,A=1.000000)" (.debug_duration _bs)))))
    (:then_1
      ;[0.08361 0.15 0.01979 0.5] PLAY_SPLASH
      (Development|PrintString "PLAY_SPLASH" true true "(R=0.000000,G=0.660000,B=1.000000,A=1.000000)" (.debug_duration (Variables|Default|GetBS)))
      (Class|PlayerController|ActivateTouchInterface _returnvalue)
      (bind _returnvalue_2 (UserInterface|CreateWidget "/Game/ART/UI/WIDGETS/WDGT_SPLASH.WDGT_SPLASH_C" _returnvalue))
      (UserInterface|Viewport|AddtoPlayerScreen _returnvalue_2)
      (Input|SetInputModeUIOnly _returnvalue 0 "DoNotLock" false)
      (Utilities|FlowControl|Delay 1.0)
      (CallFunction|NextLevel))))

(fn ConstructionScript)